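; BP_Moving_Mesh is a self-driving vehicle, filed under enemy AI models, that follows a spline at constant throttle.
; Each tick it finds spline actors and Getlane uses the first one to compute steering.
; Getlane projects a speed-scaled look-ahead along the spline tangent, snaps it to the spline, and maps the yaw error to steering input.
; Getcurrentcarspeed supplies forward speed in km/h, so faster driving looks further ahead.
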(event `self.ReceiveTick`
  (params (DeltaSeconds :type "Float (single-precision)"))
  (bind _outactors (`GameplayStatics.GetAllActorsOfClass` null))
  (bind _steering (`self.getlane` _outactors))
  (`self.SetSteeringInput` (`self.VehicleMovementComponent`) _steering)
  (`self.SetThrottleInput` (`self.VehicleMovementComponent`) 0.3))

(fn `getcurrentcarspeed`
  (returns (Speed :type "Float (double-precision)"))
  (return (* (`self.GetForwardSpeed` (`self.VehicleMovementComponent`)) 0.036)))

(fn `getlane`
  (params (Splines :type "Array of Object Object Reference"))
  (returns (steering :type "Float (double-precision)"))
  (bind _returnvalue (`Actor.K2_GetActorLocation`))
  (bind _spline (`/Game/_Enemy_AI/EnemyModels/Modular_01/BP_Moving_Mesh.Spline` (`|GetArrayItem` Splines)))
  (bind (_returnvalue_roll _returnvalue_pitch _returnvalue_yaw) (`KismetMathLibrary.BreakRotator` (`KismetMathLibrary.NormalizedDeltaRotator` (`KismetMathLibrary.FindLookAtRotation` _returnvalue (`SplineComponent.FindLocationClosestToWorldLocation` _spline (+ (* (`KismetMathLibrary.Normal` (`SplineComponent.FindTangentClosestToWorldLocation` _spline _returnvalue "World")) (`KismetMathLibrary.MapRangeClamped` (`self.getcurrentcarspeed`) 20.0 80.0 50.0 500.0)) _returnvalue) "World")) (`Actor.K2_GetActorRotation`))))
  (return (`KismetMathLibrary.MapRangeClamped` _returnvalue_yaw -90.0 90.0 -1.0 1.0)))

(fn `UserConstructionScript`)