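; Projectile actor fired by enemies or the player that damages the opposing side's hitbox, spawns a hit effect and destroys itself.
; Its owner, captured at construction, selects the target side, and Tick polls the mesh's overlapping components for player or living-enemy hitboxes.
; A looping timer raises gravity scale once travel exceeds Range, dropping the projectile.
; A box collision hit disables mesh overlaps and destroys it after a short delay.
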(event `self.ReceiveBeginPlay`
  ;[1 1 1] Each 0.05 second calculate distance from the start. Drop the projectile on the floor, if distance > Range
  (set `self.StartPoint` (`self.K2_GetActorLocation`))
  (`KismetSystemLibrary.K2_SetTimerDelegate` (delegate `DistanceFromStart`) 0.05 true))

(event `DistanceFromStart`
  ;[1 1 1] Each 0.05 second calculate distance from the start. Drop the projectile on the floor, if distance > Range
  (if (>= (`KismetMathLibrary.VSize` (- (`self.StartPoint`) (`self.K2_GetActorLocation`))) (`self.Range`))
    (set `ProjectileMovementComponent.ProjectileGravityScale` 5.0 (`self.ProjectileMovement`))))

(event `self.Box.OnComponentHit`
  (params (HitComponent :type "PrimitiveComponent Object Reference") (OtherActor :type "Actor Object Reference") (OtherComp :type "PrimitiveComponent Object Reference") (NormalImpulse :type "Vector Structure") (Hit :type "HitResult Structure (by ref)"))
  ;[1 1 1] Destroy on hit world static
  (set `PrimitiveComponent.bGenerateOverlapEvents` false (`self.StaticMesh`))
  (`KismetSystemLibrary.Delay` 0.5)
  (`self.K2_DestroyActor`))

(event `self.ReceiveTick`
  (params (DeltaSeconds :type "Float (single-precision)"))
  (bind _projectileowner (`self.ProjectileOwner`))
  ;[1 1 1] If projectile fired by enemy, destroy on hit player's hitbox
  (cast `/Game/_EnemyAIConstructor/Constructor/Blueprints/AI/BP_Enemy` _projectileowner
    (:`then`
      (bind _yes (`self.PlayerOverlapped`))
      (if _yes
        (`GameplayStatics.ApplyDamage` (`/Game/_EnemyAIConstructor/Constructor/Blueprints/Utility/BFL_UtilitiesLibrary.GetPlayer`) (`self.Damage`))
        (`GameplayStatics.SpawnEmitterAtLocation` (`self.TypeOfHitEffect`) (`SceneComponent.K2_GetComponentLocation` (`self.Box`)) :!label _label)
        (`self.K2_DestroyActor`)))
    (:`CastFailed`
      ;[1 1 1] If projectile fired by player, destroy on hit enemy's hitbox
      (cast `/Game/_EnemyAIConstructor/Constructor/Blueprints/Character/BP_CharacterBaseClass` _projectileowner)
      (bind _enemy (`self.EnemyOverlapped`))
      (if (!= _enemy null)
        (`GameplayStatics.ApplyDamage` _enemy (`self.Damage`))
        (goto _label)))))

(fn `EnemyOverlapped`
  (returns (Enemy :type "Actor Object Reference"))
  ;[1 1 1] Return reference to overlapped enemy
  (for _array_element (`PrimitiveComponent.GetOverlappingComponents` (`self.StaticMesh`))
    (bind _asbp_enemy (cast `/Game/_EnemyAIConstructor/Constructor/Blueprints/AI/BP_Enemy` (`ActorComponent.GetOwner` _array_element)))
    (if (and (== (`/Game/_EnemyAIConstructor/Constructor/Blueprints/AI/BP_Enemy.HitBox` _asbp_enemy) _array_element) (not (`/Game/_EnemyAIConstructor/Constructor/Blueprints/AI/BP_Enemy.EnemyIsDead` _asbp_enemy)))
      (return _asbp_enemy)))
  (return null))

(fn `PlayerOverlapped`
  (returns (Yes :type Boolean))
  ;[1 1 1] Return true if Projectile mesh overlap player
  (return (`KismetArrayLibrary.Array_Contains` (`PrimitiveComponent.GetOverlappingComponents` (`self.StaticMesh`)) (`/Game/_EnemyAIConstructor/Constructor/Blueprints/Utility/BFL_UtilitiesLibrary.GetPlayersHitBox`))))

(fn `UserConstructionScript`
  (set `self.ProjectileOwner` (`self.GetOwner`)))